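; BP_ZoneBlockKey is a puzzle blocker in the GettingKey set that burns away when the player uses a specific item on it from close range.
; UseItem checks the selected item and player distance, then reveals the particle effect and spawns a scaled-up BP_WarmthTrigger at the actor's transform with its warmth type set.
; A timer lasting TimeToBurnDown then destroys both the warmth trigger and the blocker.
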(event Custom|Destroy%20Actor
  (Actor|DestroyActor (stale EventUseItem _returnvalue_2))
  (Actor|DestroyActor))

(event EventBeginPlay
  (|CallParentFunction) ; This node is disabled and will not be called.\nDrag off pins to build functionality.
)

(event Collision|EventActorBeginOverlap
  (params (OtherActor :type Actor%20Object%20Reference))
  (|CallParentFunction OtherActor) ; This node is disabled and will not be called.\nDrag off pins to build functionality.
)

(event EventTick
  (params (DeltaSeconds :type Float%20%28single-precision%29))
  (|CallParentFunction DeltaSeconds) ; This node is disabled and will not be called.\nDrag off pins to build functionality.
)

(event EventUseItem
  (params (SelectedItem :type InventoryEnum%20Enum :default "NewEnumerator0"))
  (bind _returnvalue (Transformation|GetActorTransform))
  (if (and (Utilities|Enum|Equal(Enum) SelectedItem "NewEnumerator1") (<= (Transformation|GetDistanceTo (Game|GetPlayerCharacter 0) self) 3e+02))
    (Rendering|SetVisibility (Variables|Default|GetParticleSystem) true false)
    (bind _returnvalue_2 (Game|SpawnActorfromClass "/Game/ProjectResources/BluePrints/WarmthSystem/BP_WarmthTrigger.BP_WarmthTrigger_C" (Math|Transform|MakeTransform (.location _returnvalue) (.rotation _returnvalue) "10.000000,10.000000,10.000000") "Undefined" 0 0))
    (Variables|/Game/ProjectResources/BluePrints/WarmthSystem/BP_WarmthTrigger.BP_WarmthTrigger_C|SetEWarmth _returnvalue_2 "NewEnumerator0")
    (Utilities|Time|SetTimerbyEvent (delegate Custom|Destroy%20Actor) (Variables|Default|GetTimeToBurnDown))))

(fn ConstructionScript
  (|CallParentFunction))