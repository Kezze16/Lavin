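; BP_WiresEnd is the end piece of a wire in the attaching-wires puzzle, with a blue, green or red type.
; On BeginPlay it sets the WireEnd component's material to match its EWires value.
; When interacted with, it finds every actor implementing BPI_Puzzle and sends each a ClickedMessage with itself as the argument.
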(event EventBeginPlay
  (|CallParentFunction)
  ;[1 1 1] Setting Material Depending on Type
  (Rendering|Material|SetMaterial (Variables|Default|GetWireEnd) 0 (Utilities|Select :Index (Variables|Default|GetEWires) :NewEnumerator0 "/Game/ProjectResources/Art/Materials/M_Blue.M_Blue" :NewEnumerator1 "/Game/ProjectResources/Art/Materials/M_Green.M_Green" :NewEnumerator2 "/Game/ProjectResources/Art/Materials/M_Red.M_Red")))

(event Collision|EventActorBeginOverlap
  (params (OtherActor :type Actor%20Object%20Reference))
  (|CallParentFunction OtherActor) ; This node is disabled and will not be called.\nDrag off pins to build functionality.
)

(event EventTick
  (params (DeltaSeconds :type Float%20%28single-precision%29))
  (|CallParentFunction DeltaSeconds))

(event EventInteract
  (bind _outactors (Actor|GetAllActorswithInterface "/Game/ProjectResources/BluePrints/Interfaces/BPI_Puzzle.BPI_Puzzle_C"))
  (for _array_element _outactors
    (Class|BPIPuzzle|Clicked(Message) _array_element self)))

(fn ConstructionScript
  (|CallParentFunction))