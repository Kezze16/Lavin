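; BP_WireFrame is the lever-equipped frame for the wire-attaching puzzle, with an emissive status color.
; BeginPlay creates a dynamic material instance on the static mesh, and OnPuzzleComplete turns its color green.
; Interact checks WirePuzzleComplete on the first-person game mode to choose between two timeline-driven lever rotations.
; When complete, the lever swings fully and calls OnLeverPulled on BP_ZoneBlock1; otherwise it plays only a short movement.
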(event Custom|OnPuzzleComplete
  (Rendering|Material|SetVectorParameterValue (Variables|Default|GetDynamicMaterial) "Color" "(R=0.025849,G=0.465278,B=0.079957,A=1.000000)" :!class /Script/Engine.MaterialInstanceDynamic))

(event EventBeginPlay
  (|CallParentFunction)
  (bind _returnvalue (Rendering|Material|CreateDynamicMaterialInstance (Variables|Default|GetStaticMesh) 0 "/Engine/ArtTools/RenderToTexture/Materials/Debug/M_Emissive_Color.M_Emissive_Color" "None" :!class /Script/Engine.PrimitiveComponent))
  (bind _output_get (Variables|Default|SetDynamicMaterial _returnvalue))
  (Rendering|Material|SetMaterial (Variables|Default|GetStaticMesh) 0 _output_get))

(event Collision|EventActorBeginOverlap
  (params (OtherActor :type Actor%20Object%20Reference))
  (|CallParentFunction OtherActor) ; This node is disabled and will not be called.\nDrag off pins to build functionality.
)

(event EventTick
  (params (DeltaSeconds :type Float%20%28single-precision%29))
  (|CallParentFunction DeltaSeconds) ; This node is disabled and will not be called.\nDrag off pins to build functionality.
)

(event EventInteract
  (bind _asbp_first_person_game_mode (Utilities|Casting|CastToBP_FirstPersonGameMode (Game|GetGameMode)))
  (if (Variables|/Game/FirstPerson/Blueprints/BP_FirstPersonGameMode.BP_FirstPersonGameMode_C|GetWirePuzzleComplete _asbp_first_person_game_mode)
    (bind _newtrack_0 (Timeline|Lever Play)
      (:Update
        (Transformation|SetRelativeRotation (Variables|Default|GetSM_FuseLadderInteract) (Math|Rotator|Lerp(Rotator) "180.000000,0.000000,-180.000000" "0.000000,0.000000,-180.000000" _newtrack_0) false false))
      (:Finished
        (bind _returnvalue (Actor|GetActorOfClass "/Game/ProjectResources/BluePrints/Puzzles/AttatchingWires/BP_ZoneBlock1.BP_ZoneBlock1_C"))
        (Default|OnLeverPulled _returnvalue)))
    (else
      (bind _newtrack_0_2 (Timeline|Timeline PlayFromStart)
        (:Update
          (Transformation|SetRelativeRotation (Variables|Default|GetSM_FuseLadderInteract) (Math|Rotator|Lerp(Rotator) "180.000000,0.000000,-180.000000" "140.000000,0.000000,-180.000000" _newtrack_0_2) false false))))))

(fn ConstructionScript
  (|CallParentFunction))