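; BP_WiresStart is the start point of a colored wire in the wire-attaching puzzle.
; On BeginPlay it tints its mesh and cable blue, green or red from its EWires type.
; Interact toggles selection; while selected, Clicked attaches the cable end to the given actor's WireEnd socket and deselects.
; It then reports both wire types to BP_FirstPersonGameMode via WirePuzzleSetTrue to track puzzle progress.
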(event EventBeginPlay
  (bind _ewires (Variables|Default|GetEWires))
  (bind _returnvalue (Utilities|Select :Index _ewires :NewEnumerator0 "/Game/ProjectResources/Art/Materials/M_Blue.M_Blue" :NewEnumerator1 "/Game/ProjectResources/Art/Materials/M_Green.M_Green" :NewEnumerator2 "/Game/ProjectResources/Art/Materials/M_Red.M_Red"))
  (|CallParentFunction)
  ;[1 1 1] Setting Material Depending on Type
  (Rendering|Material|SetMaterial (Variables|Default|GetStaticMesh) 0 _returnvalue)
  (Rendering|Material|SetMaterial (Variables|Default|GetCable) 0 _returnvalue))

(event Collision|EventActorBeginOverlap
  (params (OtherActor :type Actor%20Object%20Reference))
  (|CallParentFunction OtherActor) ; This node is disabled and will not be called.\nDrag off pins to build functionality.
)

(event EventTick
  (params (DeltaSeconds :type Float%20%28single-precision%29))
  (|CallParentFunction DeltaSeconds))

(event EventInteract
  ;[1 1 1] Selecting Actor
  (Variables|Default|SetIsSelected (not (Variables|Default|GetIsSelected))))

(event EventClicked
  (params (Actor :type BP%20Wires%20End%20Object%20Reference))
  ;[1 1 1] If Selected when clicking connector connect to it
  (if (Variables|Default|GetIsSelected)
    (Class|CableComponent|SetAttachEndto (Variables|Default|GetCable) Actor "WireEnd" "WireSocket")
    ;[1 1 1] Tell Puzzle Manager that it cable has been connected
    (bind _asbp_first_person_game_mode (Utilities|Casting|CastToBP_FirstPersonGameMode (Game|GetGameMode)))
    (Default|WirePuzzleSetTrue _asbp_first_person_game_mode (Variables|Default|GetEWires) (Variables|/Game/ProjectResources/BluePrints/Puzzles/AttatchingWires/BP_WiresEnd.BP_WiresEnd_C|GetEWires Actor))
    (Variables|Default|SetIsSelected false)))

(fn ConstructionScript
  (|CallParentFunction))