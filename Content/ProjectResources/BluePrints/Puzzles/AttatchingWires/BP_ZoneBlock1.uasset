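; Blocking-zone puzzle actor that takes two placed dynamite charges and blows itself up after a lever pull.
; On BeginPlay it caches the dynamite materials and shows both charges as outline placeholders.
; Using the matching item restores one charge's materials and reveals its cable, with the second also setting DynamiteInPlace on the game mode.
; OnLeverPulled starts a timed fuse, then Explode spawns effects and sound and destroys the actor.
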(event Custom|OnLeverPulled
  (Utilities|Time|SetTimerbyEvent (delegate Custom|Explode) 7.0))

(event Custom|Explode
  (bind _returnvalue (Transformation|GetActorLocation))
  (for _index (range 0 3)
    (Effects|SpawnEmitteratLocation "/Game/StarterContent/Particles/P_Explosion.P_Explosion" (Math|Vector|MakeVector (- (.x _returnvalue) 3.5e+02) (.y _returnvalue) (.z _returnvalue)) "0, 0, 0" "15.000000,15.000000,15.000000")
    (Audio|PlaySoundatLocation "/Game/ProjectResources/Sounds/Explostion.Explostion" (Transformation|GetActorLocation) "0, 0, 0" 1.0 1.0 0.0 0 0 0 0))
  (Utilities|FlowControl|Delay 0.2)
  (Actor|DestroyActor))

(event EventBeginPlay
  ;[1 1 1] Storing mats and setting up placeholders
  (Variables|Default|SetDynamiteMats (Rendering|Material|GetMaterials (Variables|Default|GetDynamite1)))
  (for _index (range 0 1)
    (Rendering|Material|SetMaterial (Variables|Default|GetDynamite2) _index "/Game/ProjectResources/Art/Materials/M_Outline.M_Outline")
    (for _index_2 (range 0 1)
      (Rendering|Material|SetMaterial (Variables|Default|GetDynamite1) _index_2 "/Game/ProjectResources/Art/Materials/M_Outline.M_Outline"))))

(event Collision|EventActorBeginOverlap
  (params (OtherActor :type Actor%20Object%20Reference)))

(event EventTick
  (params (DeltaSeconds :type Float%20%28single-precision%29)))

(event EventUseItem
  (params (SelectedItem :type InventoryEnum%20Enum :default "NewEnumerator0"))
  (if (Utilities|Enum|Equal(Enum) SelectedItem "NewEnumerator10")
    (if (Variables|Default|GetGotDynamite1)
      (for (_array_element _array_index) (Variables|Default|GetDynamiteMats)
        (Rendering|Material|SetMaterial (Variables|Default|GetDynamite2) _array_index _array_element)
        (Rendering|SetVisibility (Variables|Default|GetCable1) true false)
        (bind _asbp_first_person_game_mode (Utilities|Casting|CastToBP_FirstPersonGameMode (Game|GetGameMode)))
        (Variables|/Game/FirstPerson/Blueprints/BP_FirstPersonGameMode.BP_FirstPersonGameMode_C|SetDynamiteInPlace _asbp_first_person_game_mode true))
      (else
        (for (_array_element_2 _array_index_2) (Variables|Default|GetDynamiteMats)
          (Rendering|Material|SetMaterial (Variables|Default|GetDynamite1) _array_index_2 _array_element_2)
          (Rendering|SetVisibility (Variables|Default|GetCable) true false)
          (Variables|Default|SetGotDynamite1 true))))))

(fn ConstructionScript)

(fn NewFunction
  (for _index (range (Utilities|Array|LastIndex (Variables|Default|GetDynamiteMats)) 0)
    (Rendering|Material|SetMaterial (Variables|Default|GetDynamite2) _index "/Game/ProjectResources/Art/Materials/M_Outline.M_Outline")))