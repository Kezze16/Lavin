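; BP_Lockpicking is the lockpicking puzzle actor, managing setup, knife motion and completion.
; Spawn shows the W_Lockpicking widget, picks a random correct pick yaw and disables first-person character input through a FlipFlop toggle.
; Two timelines rotate the knife pivot for move attempts and resets.
; Unlocked removes the widget, clears IsLocked, toggles input back on and destroys the actor.
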(event Custom|Unlocked
  (Widget|RemovefromParent (Variables|Default|GetW_Lockpick))
  (Variables|Default|SetIsLocked false)
  (CallFunction|ToggleCharacterInput)
  (Actor|DestroyActor))

(event Custom|TryToMoveKnife
  (bind _newtrack_0 (Timeline|Timeline PlayFromStart)
    (:Update
      (Transformation|SetRelativeRotation (Variables|Default|GetKnifePivot) (Math|Rotator|Lerp(Rotator) "0.000000,-108.000000,90.000000" "0.000000,-108.000000,100.000000" _newtrack_0) false false))))

(event Custom|ResetKnifeRot
  (bind _reset (Timeline|Timeline_0 Play)
    (:Update
      (Transformation|SetRelativeRotation (Variables|Default|GetKnifePivot) (Math|Rotator|Lerp(Rotator) (Variables|/Script/Engine.SceneComponent|GetRelativeRotation (Variables|Default|GetKnifePivot)) "0.000000,-108.000000,90.000000" _reset) false false))))

(event Custom|Spawn
  (bind _returnvalue (UserInterface|CreateWidget "/Game/ProjectResources/UI/LockPicking/W_Lockpicking.W_Lockpicking_C"))
  (bind _output_get (Variables|Default|SetW_Lockpick _returnvalue))
  (UserInterface|Viewport|AddtoViewport _output_get 0)
  (Variables|Default|SetCorrectRotationPick (Math|Rotator|MakeRotator 0.0 (Math|Random|RandomFloatinRange -9e+01 9e+01) 0.0))
  (CallFunction|ToggleCharacterInput))

(event Custom|ToggleCharacterInput
  (bind _returnvalue (Game|GetPlayerController 0))
  ;[1 1 1] Toggle Input for Character
  (bind _returnvalue_2 (Actor|GetActorOfClass "/Game/FirstPerson/Blueprints/BP_FirstPersonCharacter.BP_FirstPersonCharacter_C"))
  (Utilities|FlowControl|FlipFlop
    (:A
      (Input|DisableInput _returnvalue_2 _returnvalue))
    (:B
      (Input|EnableInput _returnvalue_2 _returnvalue))))

(event Collision|EventActorBeginOverlap
  (params (OtherActor :type Actor%20Object%20Reference))
  (|CallParentFunction OtherActor) ; This node is disabled and will not be called.\nDrag off pins to build functionality.
)

(event EventTick
  (params (DeltaSeconds :type Float%20%28single-precision%29))
  (|CallParentFunction DeltaSeconds) ; This node is disabled and will not be called.\nDrag off pins to build functionality.
)

(fn ConstructionScript
  (|CallParentFunction))