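; Interactable chest actor that launches a lockpicking minigame or swings open and closed.
; On Interact, if it is locked and the inventory map holds a lockpick, it spawns and starts BP_Lockpicking at the Lock component, once only.
; Otherwise, including when locked without a lockpick, a FlipFlop plays or reverses a Timeline that rotates the mesh.
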(event EventBeginPlay
  (|CallParentFunction) ; This node is disabled and will not be called.\nDrag off pins to build functionality.
)

(event Collision|EventActorBeginOverlap
  (params (OtherActor :type Actor%20Object%20Reference))
  (|CallParentFunction OtherActor) ; This node is disabled and will not be called.\nDrag off pins to build functionality.
)

(event EventTick
  (params (DeltaSeconds :type Float%20%28single-precision%29))
  (|CallParentFunction DeltaSeconds) ; This node is disabled and will not be called.\nDrag off pins to build functionality.
)

(event EventInteract
  ;[1 1 1] Checking if Lockpick is in inventory
  (if (and (Variables|Default|GetIsLocked) (>= (.Value (Utilities|Map|Find (Variables|Default|GetInventoryMap) (Variables|Default|GetInventoryItems))) 1))
    ;[1 1 1] Spawning Lockpick BP
    (Utilities|FlowControl|DoOnce false
      (:Completed
        (bind _returnvalue (Game|SpawnActorfromClass "/Game/ProjectResources/BluePrints/Puzzles/Lockpicking/BP_Lockpicking.BP_Lockpicking_C" (Math|Transform|MakeTransform (.location (Transformation|GetWorldTransform (Variables|Default|GetLock))) "0.000000,180.000000,0.000000" "0.800000,0.800000,0.800000") "Undefined" 0 0))
        (Default|Spawn _returnvalue)))
    (else
      ;[1 1 1] Chest Open/Close Anim
      (Utilities|FlowControl|FlipFlop
        (:A
          (bind _newtrack_0 (Timeline|Timeline Play)
            (:Update
              (Transformation|SetRelativeRotation (Variables|Default|GetStaticMesh1) (Math|Rotator|Lerp(Rotator) "0.000000,0.000000,-90.000000" "0.000000,0.000000,45.000000" _newtrack_0) false false))))
        (:B
          (Timeline|Timeline Reverse))))))

(fn ConstructionScript
  (|CallParentFunction))