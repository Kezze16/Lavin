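; BP_RadioBox is the radio box in the turning-on-power puzzle folder that ends the game when interacted with.
; Interact spawns an enlarged BP_WarmthTrigger at the box with its warmth enum set, disables player input and plays the EndCinematic level sequence.
; A fixed timer, independent of the sequence's finish, then fires GameCompleted to open the main menu level.
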(event Custom|GameCompleted
  (Game|OpenLevel(byObjectReference) "/Game/ProjectResources/Maps/GameMaps/MainMenuScene.MainMenuScene"))

(event EventBeginPlay)

(event Collision|EventActorBeginOverlap
  (params (OtherActor :type Actor%20Object%20Reference)))

(event EventTick
  (params (DeltaSeconds :type Float%20%28single-precision%29)))

(event EventInteract
  (bind _returnvalue (Transformation|GetActorTransform))
  (bind _returnvalue_2 (Game|SpawnActorfromClass "/Game/ProjectResources/BluePrints/WarmthSystem/BP_WarmthTrigger.BP_WarmthTrigger_C" (Math|Transform|MakeTransform (.location _returnvalue) (.rotation _returnvalue) "10.000000,10.000000,10.000000") "Undefined" 0 0))
  (Variables|/Game/ProjectResources/BluePrints/WarmthSystem/BP_WarmthTrigger.BP_WarmthTrigger_C|SetEWarmth _returnvalue_2 "NewEnumerator0")
  (Input|DisableInput (Game|GetPlayerCharacter 0) (Game|GetPlayerController 0))
  (bind _returnvalue_3 (Sequencer|Player|CreateLevelSequencePlayer "/Game/ProjectResources/Cinnematic/EndCinematic.EndCinematic"))
  (Sequencer|Player|Play _returnvalue_3 :!class /Script/MovieScene.MovieSceneSequencePlayer)
  (Utilities|Time|SetTimerbyEvent (delegate Custom|GameCompleted) 22.5))

(fn ConstructionScript)