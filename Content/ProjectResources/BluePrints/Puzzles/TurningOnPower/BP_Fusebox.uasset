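; Fusebox puzzle actor for turning on power, with three fuse slots filled through item use.
; BeginPlay caches Fuse1's materials, gives all three fuse meshes an outline placeholder material and creates a dynamic blinking material.
; UseItem with the matching item loops over the cached materials, applying each to the mesh selected by FuseAmount and incrementing that count.
; At three or more, it calls FusesInPlace on the game mode and turns the blinking material green.
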(event EventBeginPlay
  ;[1 1 1] Storing mats and setting up placeholders
  (bind _returnvalue (Rendering|Material|CreateDynamicMaterialInstance "/Game/ProjectResources/Art/Materials/M_Blinking_Fuses.M_Blinking_Fuses" "None" "None" :!class /Script/Engine.KismetMaterialLibrary))
  (Variables|Default|SetBlinkingMat _returnvalue)
  (Variables|Default|SetFuseMats (Rendering|Material|GetMaterials (Variables|Default|GetFuse1)))
  (for _index (range 0 1)
    (Rendering|Material|SetMaterial (Variables|Default|GetFuse1) _index "/Game/ProjectResources/Art/Materials/M_Outline.M_Outline")
    (for _index_2 (range 0 1)
      (Rendering|Material|SetMaterial (Variables|Default|GetFuse2) _index_2 "/Game/ProjectResources/Art/Materials/M_Outline.M_Outline")
      (for _index_3 (range 0 1)
        (Rendering|Material|SetMaterial (Variables|Default|GetFuse3) _index_3 "/Game/ProjectResources/Art/Materials/M_Outline.M_Outline")))))

(event Collision|EventActorBeginOverlap
  (params (OtherActor :type Actor%20Object%20Reference)))

(event EventTick
  (params (DeltaSeconds :type Float%20%28single-precision%29)))

(event EventUseItem
  (params (SelectedItem :type InventoryEnum%20Enum :default "NewEnumerator0"))
  (if (Utilities|Enum|Equal(Enum) SelectedItem "NewEnumerator8")
    (for _array_element (Variables|Default|GetFuseMats)
      (Rendering|Material|SetMaterial (Utilities|Select :Index (Variables|Default|GetFuseAmount) :Option%200 (Variables|Default|GetFuse1) :Option%201 (Variables|Default|GetFuse2) :Option%202 (Variables|Default|GetFuse3)) 0 _array_element)
      (bind _result (Math|Integer|IncrementInt (Variables|Default|GetFuseAmount))
        (:%20%20
          (bind _output_get (Variables|Default|SetFuseAmount _result))
          (if (>= _output_get 3)
            (bind _asbp_first_person_game_mode (Utilities|Casting|CastToBP_FirstPersonGameMode (Game|GetGameMode)))
            (Default|FusesinPlace _asbp_first_person_game_mode)
            (Rendering|Material|SetVectorParameterValue (Variables|Default|GetBlinkingMat) "Color" "(R=0.042007,G=0.791667,B=0.000000,A=1.000000)" :!class /Script/Engine.MaterialInstanceDynamic)))))))

(fn ConstructionScript)