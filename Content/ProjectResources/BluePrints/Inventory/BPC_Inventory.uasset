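; BPC_Inventory is the player's inventory component, storing item counts and toggling the W_Inventory screen, cursor and input mode via IA_Inventory.
; Add events map item enums to DT_Item rows, which key a count map.
; Lantern Refill skips the map and adds 80% of max fuel to BPC_Lantern.
; Removal handles only Lantern Fuel, dropping empty entries and recreating the widget to refresh it.
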(event Custom|Refresh%20Widget
  (bind _returnvalue (Game|GetPlayerController 0))
  ;[1 1 1] Refresh Widget
  (Widget|RemovefromParent (Variables|Default|GetInventoryWidget))
  (Variables|Default|SetbIsInventoryOpen false)
  (Variables|/Script/Engine.PlayerController|SetbShowMouseCursor _returnvalue false)
  (Input|SetInputModeGameOnly _returnvalue false)
  (bind _returnvalue_2 (UserInterface|CreateWidget "/Game/ProjectResources/UI/Inventory/W_Inventory.W_Inventory_C"))
  (bind _output_get (Variables|Default|SetInventoryWidget _returnvalue_2))
  (UserInterface|Viewport|AddtoViewport _output_get 0)
  (Variables|Default|SetbIsInventoryOpen true)
  (Input|SetInputModeGameandUI _returnvalue _output_get "DoNotLock" false false)
  (Variables|/Script/Engine.PlayerController|SetbShowMouseCursor _returnvalue true))

(event Custom|RemoveInventoryItem
  (params (Inventory%20Item%20Enum :type InventoryEnum%20Enum :default "NewEnumerator0"))
  ;[1 1 1] Removing Item From Inventory
  (CallFunction|RemoveItems Inventory%20Item%20Enum))

(event Custom|AddInventoryItem
  (params (InventoryItemEnum :type InventoryEnum%20Enum :default "NewEnumerator0"))
  ;[1 1 1] Adding Item to Inventory
  (CallFunction|PopulateInventory InventoryItemEnum))

(event Input|EnhancedActionEvents|EnhancedInputActionIA_Inventory
  (params (ActionValue :type Boolean) (ElapsedSeconds :type Float%20%28double-precision%29) (TriggeredSeconds :type Float%20%28double-precision%29) (InputAction :type Input%20Action%20Object%20Reference :default "/Game/FirstPerson/Input/Actions/IA_Inventory.IA_Inventory"))
  (bind _returnvalue (Game|GetPlayerController 0))
  ;[1 1 1] Adding Widget to Screen
  (:Triggered
    (if (Variables|Default|GetbIsInventoryOpen)
      (Widget|RemovefromParent (Variables|Default|GetInventoryWidget))
      (Variables|Default|SetbIsInventoryOpen false)
      (Variables|/Script/Engine.PlayerController|SetbShowMouseCursor _returnvalue false)
      (Input|SetInputModeGameOnly _returnvalue false)
      (else
        (bind _returnvalue_2 (UserInterface|CreateWidget "/Game/ProjectResources/UI/Inventory/W_Inventory.W_Inventory_C"))
        (bind _output_get (Variables|Default|SetInventoryWidget _returnvalue_2))
        (UserInterface|Viewport|AddtoViewport _output_get 0)
        (Variables|Default|SetbIsInventoryOpen true)
        (Input|SetInputModeGameandUI _returnvalue _output_get "DoNotLock" false false)
        (Variables|/Script/Engine.PlayerController|SetbShowMouseCursor _returnvalue true)))))

(fn UpdateUI
  (params (Item :type Item%20Type%20Structure))
  (bind _inventorymap (Variables|Default|GetInventoryMap))
  (bind (_value _returnvalue) (Utilities|Map|Find _inventorymap Item))
  ;[1 1 1] Adding new item or updating item amount in Map
  (if _returnvalue
    (Utilities|Map|Add (Variables|Default|GetInventoryMap) Item (+ _value 1))
    (else
      (Utilities|Map|Add (Variables|Default|GetInventoryMap) Item 1))))

(fn PopulateInventory
  (params (EItemType :type InventoryEnum%20Enum :default "NewEnumerator0"))
  (bind _returnvalue (Game|GetPlayerCharacter 0))
  (bind _returnvalue_2 (Actor|GetComponentbyClass _returnvalue "/Game/ProjectResources/BluePrints/BPC_Lantern.BPC_Lantern_C"))
  ;[1 1 1] Finding correct DT row based in Item Type Enum
  (switch Utilities|FlowControl|Switch|SwitchonInventoryEnum EItemType
    (:NewEnumerator0
      (Variables|Default|SetName "Fuel")
      (bind _returnvalue_3 (Utilities|GetDataTableRow "/Game/ProjectResources/BluePrints/Inventory/ENum/DT_Item.DT_Item" (Variables|Default|GetName) :!label _label)
        (:then
          (Variables|Default|SetEItem (.EItem (Utilities|Struct|BreakItemType _returnvalue_3)))
          (CallFunction|UpdateUI _returnvalue_3))))
    (:NewEnumerator1
      (Variables|Default|SetName "Lantern")
      (goto _label))
    (:NewEnumerator2
      (Default|AddFuel _returnvalue_2 (* (Variables|/Game/ProjectResources/BluePrints/BPC_Lantern.BPC_Lantern_C|GetMaxFuel _returnvalue_2) 0.8)))))

(fn RemoveItems
  (params (Item :type InventoryEnum%20Enum :default "NewEnumerator0"))
  ;[1 1 1] Finding the row for modifying
  (switch Utilities|FlowControl|Switch|SwitchonInventoryEnum Item
    (:NewEnumerator0
      (Variables|Default|SetName "Fuel")
      (bind _returnvalue (Utilities|GetDataTableRow "/Game/ProjectResources/BluePrints/Inventory/ENum/DT_Item.DT_Item" (Variables|Default|GetName))
        (:then
          ;[1 1 1] Finding The Associated "amount" of that DT Row and adding/subtracting from that
          (if (.ReturnValue (Utilities|Map|Find (Variables|Default|GetInventoryMap) _returnvalue))
            (Utilities|Map|Add (Variables|Default|GetInventoryMap) _returnvalue (- (.Value (Utilities|Map|Find (Variables|Default|GetInventoryMap) _returnvalue)) 1))
            ;[1 1 1] If "Amount" is 0 or less then remove the row altogether
            (if (<= (.Value (Utilities|Map|Find (Variables|Default|GetInventoryMap) _returnvalue)) 0)
              (Utilities|Map|Remove (Variables|Default|GetInventoryMap) _returnvalue))
            (CallFunction|RefreshWidget)))))))