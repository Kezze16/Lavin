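; BP_Inspect is an inventory inspection actor that the player spins around its vertical axis by click-dragging.
; Clicking and releasing ScrollCylinder toggles dragging, during which an input axis accumulates into a yaw velocity each tick.
; Tick applies that velocity as world rotation and damps it by a fixed per-frame factor above a small threshold, giving an inertial, frame-rate-dependent slowdown.
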(event OnClicked(ScrollCylinder)
  (params (TouchedComponent :type Primitive%20Component%20Object%20Reference) (ButtonPressed :type Key%20Structure :default "None"))
  (Variables|Default|SetisDragging true))

(event OnReleased(ScrollCylinder)
  (params (TouchedComponent :type Primitive%20Component%20Object%20Reference) (ButtonReleased :type Key%20Structure :default "None"))
  (Variables|Default|SetisDragging false))

(event Custom|HandleDragEvent
  (params (DeltaTime :type Float%20%28double-precision%29))
  (if (Variables|Default|GetisDragging)
    (bind _output_get (Variables|Default|SetDragSumX (- (Variables|Default|GetDragSumX) (Class|Actor|GetInputAxisKeyValue))))
    (Variables|Default|SetRotateVelocity (+ (Variables|Default|GetRotateVelocity) (* (* _output_get DeltaTime) 9e+01)))
    (else
      (Variables|Default|SetDragSumX 0.0))))

(event Custom|HandleRotation
  (params (DeltaTime :type Float%20%28double-precision%29))
  (Class|Actor|AddActorWorldRotation (Math|Rotator|MakeRotator 0.0 0.0 (* DeltaTime (Variables|Default|GetRotateVelocity))))
  (if (or (< (Variables|Default|GetRotateVelocity) -0.1) (> (Variables|Default|GetRotateVelocity) 0.1))
    (Variables|Default|SetRotateVelocity (* (Variables|Default|GetRotateVelocity) 0.95))
    (Variables|Default|SetDragSumX (* (Variables|Default|GetDragSumX) 0.95))))

(event EventBeginPlay)

(event Collision|EventActorBeginOverlap
  (params (OtherActor :type Actor%20Object%20Reference)))

(event EventTick
  (params (DeltaSeconds :type Float%20%28single-precision%29))
  (CallFunction|HandleRotation DeltaSeconds)
  (CallFunction|HandleDragEvent DeltaSeconds))

(fn ConstructionScript)