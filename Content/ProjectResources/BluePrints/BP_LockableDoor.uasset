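; BP_LockableDoor is an interactable door that stays shut until the player uses the matching inventory item on it.
; Interact plays a locked sound while IsLocked is set, otherwise a squeak and a FlipFlop that plays or reverses the DoorOpen timeline.
; The timeline lerps the DoorPivot relative rotation to swing the door open and closed.
; UseItem clears IsLocked when the selected item matches one specific enum entry.
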(event EventBeginPlay)

(event Collision|EventActorBeginOverlap
  (params (OtherActor :type Actor%20Object%20Reference)))

(event EventTick
  (params (DeltaSeconds :type Float%20%28single-precision%29)))

(event EventInteract
  (if (Variables|Default|GetbIsLocked)
    (Audio|PlaySound2D "/Game/ProjectResources/Sound/SFX/Door.Door" 1.0 1.0 0.0 0 0)
    (else
      (Audio|PlaySound2D "/Game/ProjectResources/Sound/SFX/SqueakingDoor.SqueakingDoor" 1.0 1.0 0.0 0 0)
      (Utilities|FlowControl|FlipFlop
        (:A
          (bind _newtrack_0 (Timeline|DoorOpen Play)
            (:Update
              (Transformation|SetRelativeRotation (Variables|Default|GetDoorPivot) (Math|Rotator|Lerp(Rotator) "0, 0, 0" "0.000000,125.000000,0.000000" _newtrack_0) false false))))
        (:B
          (Timeline|DoorOpen Reverse))))))

(event EventUseItem
  (params (SelectedItem :type InventoryEnum%20Enum :default "NewEnumerator0"))
  (if (Utilities|Enum|Equal(Enum) SelectedItem "NewEnumerator7")
    (Variables|Default|SetbIsLocked false)))

(fn ConstructionScript)