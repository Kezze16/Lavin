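; Player lantern component that gives light and changes the character's cold decrease rate while burning fuel.
; Pickup fills fuel, shows the lantern and fuel HUD; input toggles burning, the first-person anim state and warming rate.
; Tick drains fuel and scales point light radius and intensity with it, restoring the default rate when empty.
; Adding fuel resets the game mode timer, but the FuelIsOut call is never run.
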(event Custom|BurnFuel
  (params (Delta%20Seconds :type Float%20%28double-precision%29))
  ;[1 1 1] Fuel Drainage
  (if (<= (Variables|Default|GetCurrentFuel) 0.0)
    (Variables|Default|SetbIsBurning? false)
    (bind _asbp_first_person_character (Utilities|Casting|CastToBP_FirstPersonCharacter (Components|GetOwner)))
    (Default|SetDecreaseRate _asbp_first_person_character 1.5)
    (else
      (Variables|Default|SetCurrentFuel (Math|Float|Clamp(Float) (- (Variables|Default|GetCurrentFuel) (* Delta%20Seconds (Variables|Default|GetFuelBurnRate))) 0.0 (Variables|Default|GetMaxFuel))))))

(event Custom|AddFuel
  (params (AddedFuelAmount :type Float%20%28double-precision%29))
  ;[1 1 1] Adding Fuel
  (Variables|Default|SetCurrentFuel (+ (Variables|Default|GetCurrentFuel) AddedFuelAmount))
  (bind _asbp_first_person_game_mode (Utilities|Casting|CastToBP_FirstPersonGameMode (Game|GetGameMode)))
  (Default|ResetTimer _asbp_first_person_game_mode)
  (Development|PrintString "FuelAdded"))

(event Custom|AdjustLightLevel
  (bind _currentfuel (Variables|Default|GetCurrentFuel))
  ;[1 1 1] Simple Light Fade
  (bind _asbp_first_person_character (Utilities|Casting|CastToBP_FirstPersonCharacter (Components|GetOwner)))
  (Rendering|Lighting|SetAttenuationRadius (Variables|/Game/FirstPerson/Blueprints/BP_FirstPersonCharacter.BP_FirstPersonCharacter_C|GetPointLight _asbp_first_person_character) (* _currentfuel 5e+01))
  (Rendering|Components|Light|SetIntensity (Variables|/Game/FirstPerson/Blueprints/BP_FirstPersonCharacter.BP_FirstPersonCharacter_C|GetPointLight _asbp_first_person_character) (* _currentfuel 1e+02)))

(event Custom|PickedUp
  (Variables|Default|SetbIsBurning? true)
  (Variables|Default|SetHasLantern true)
  (Variables|Default|SetbBurnFuel? true)
  (CallFunction|HasLanternToggle)
  (Variables|Default|SetCurrentFuel (Variables|Default|GetMaxFuel))
  ;[1 1 1] Toggle Lantern Visibility on Pick Up
  (bind _asbp_first_person_character (Utilities|Casting|CastToBP_FirstPersonCharacter (Components|GetOwner)))
  (Rendering|ToggleVisibility (Variables|/Game/FirstPerson/Blueprints/BP_FirstPersonCharacter.BP_FirstPersonCharacter_C|GetLantern _asbp_first_person_character) true)
  (Widget|SetVisibility (Variables|/Game/ProjectResources/UI/HUD/W_ColdMeter.W_ColdMeter_C|GetVerticalBoxFuel (Variables|Default|GetW_HUD)) "SelfHitTestInvisible"))

(event Custom|HasLanternToggle
  ;[1 1 1] Toggle Lantern Anim
  (bind _returnvalue (Actor|GetActorOfClass "/Game/FirstPerson/Blueprints/BP_FirstPersonCharacter.BP_FirstPersonCharacter_C"))
  (bind _asfirst_person_anim_bp (Utilities|Casting|CastToFirstPerson_AnimBP (Components|SkeletalMesh|GetAnimInstance (Variables|/Game/FirstPerson/Blueprints/BP_FirstPersonCharacter.BP_FirstPersonCharacter_C|GetFirstPersonMesh _returnvalue))))
  (bind _output_get (Variables|/Game/FirstPersonArms/Animations/FirstPerson_AnimBP.FirstPerson_AnimBP_C|SetHasLantern _asfirst_person_anim_bp (not (Variables|/Game/FirstPersonArms/Animations/FirstPerson_AnimBP.FirstPerson_AnimBP_C|GetHasLantern _asfirst_person_anim_bp))))
  (if _output_get
    (bind _asbp_first_person_character (Utilities|Casting|CastToBP_FirstPersonCharacter (Components|GetOwner)))
    (Default|SetDecreaseRate _asbp_first_person_character (Variables|Default|GetLanternWarming))
    (else
      (Rendering|Components|Light|SetIntensity (Variables|/Game/FirstPerson/Blueprints/BP_FirstPersonCharacter.BP_FirstPersonCharacter_C|GetPointLight _returnvalue) 0.0)
      (bind _asbp_first_person_character_2 (Utilities|Casting|CastToBP_FirstPersonCharacter (Components|GetOwner)))
      (Default|SetDecreaseRate _asbp_first_person_character_2 1.5))))

(event Input|EnhancedActionEvents|EnhancedInputActionIA_ToggleLantern
  (params (ActionValue :type Boolean) (ElapsedSeconds :type Float%20%28double-precision%29) (TriggeredSeconds :type Float%20%28double-precision%29) (InputAction :type Input%20Action%20Object%20Reference :default "/Game/FirstPerson/Input/Actions/IA_ToggleLantern.IA_ToggleLantern"))
  ;[1 1 1] Toggle Lantern
  (:Triggered
    (if (Variables|Default|GetHasLantern)
      (if (Variables|Default|GetbBurnFuel?)
        (Variables|Default|SetbBurnFuel? false)
        (CallFunction|HasLanternToggle)
        (else
          (Variables|Default|SetbBurnFuel? true)
          (CallFunction|HasLanternToggle))))))

(event EventBeginPlay
  (bind _returnvalue (UserInterface|CreateWidget "/Game/ProjectResources/UI/HUD/W_ColdMeter.W_ColdMeter_C"))
  (bind _output_get (Variables|Default|SetW_HUD _returnvalue))
  (UserInterface|Viewport|AddtoViewport _output_get 0))

(event EventTick
  (params (DeltaSeconds :type Float%20%28single-precision%29))
  (if (Variables|Default|GetbBurnFuel?)
    (CallFunction|BurnFuel DeltaSeconds)
    (CallFunction|AdjustLightLevel)))