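; BP_WarmthTrigger is a box trigger that warms the player while overlapped, at a strength set by its EWarmth rank.
; Begin overlap picks the rank's rate and negates it into the first-person character's WarmthDecreaseRate, with Rank 1 strongest.
; End overlap clears the rank rates and resets the decrease rate to a fixed default.
; It always targets player character 0, without checking the overlapping actor, and prints debug values.
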(event OnComponentBeginOverlap(Box)
  (params (OverlappedComponent :type Primitive%20Component%20Object%20Reference) (OtherActor :type Actor%20Object%20Reference) (OtherComp :type Primitive%20Component%20Object%20Reference) (OtherBodyIndex :type Integer) (bFromSweep :type Boolean) (SweepResult :type Hit%20Result%20Structure%20%28by%20ref%29))
  ;[1 1 1] Setting up the different ranks
  (switch Utilities|FlowControl|Switch|SwitchonE_Warmth (Variables|Default|GetEWarmth)
    (:NewEnumerator0
      (Development|PrintString "1")
      (Variables|Default|SetRank1Rate 1e+01))
    (:NewEnumerator1
      (Development|PrintString "2")
      (Variables|Default|SetRank2Rate 5.0))
    (:NewEnumerator2
      (Development|PrintString "3")
      (Variables|Default|SetRank3Rate 1.0)))
  ;[1 1 1] Casting to FPC & Setting new warmth rate
  (bind _asbp_first_person_character (Utilities|Casting|CastToBP_FirstPersonCharacter (Game|GetPlayerCharacter 0)))
  (bind _output_get (Variables|Default|SetWarmingRate1 (* (+ (Variables|Default|GetRank1Rate) (Variables|Default|GetRank2Rate) (Variables|Default|GetRank3Rate)) -1.0)))
  (Variables|/Game/FirstPerson/Blueprints/BP_FirstPersonCharacter.BP_FirstPersonCharacter_C|SetWarmthDecreaseRate _asbp_first_person_character _output_get)
  (Development|PrintString (Utilities|String|ToString(Float) (* (+ (Variables|Default|GetRank1Rate) (Variables|Default|GetRank2Rate) (Variables|Default|GetRank3Rate)) -1.0))))

(event OnComponentEndOverlap(Box)
  (params (OverlappedComponent :type Primitive%20Component%20Object%20Reference) (OtherActor :type Actor%20Object%20Reference) (OtherComp :type Primitive%20Component%20Object%20Reference) (OtherBodyIndex :type Integer))
  (Variables|Default|SetWarmingRate1 1.0)
  (Variables|Default|SetRank1Rate 0.0)
  (Variables|Default|SetRank2Rate 0.0)
  (Variables|Default|SetRank3Rate 0.0)
  ;[1 1 1] Casting to FPC & Setting new warmth rate
  (Variables|/Game/FirstPerson/Blueprints/BP_FirstPersonCharacter.BP_FirstPersonCharacter_C|SetWarmthDecreaseRate (stale OnComponentBeginOverlap(Box) _asbp_first_person_character) (stale OnComponentBeginOverlap(Box) _output_get))
  (Development|PrintString (Utilities|String|ToString(Float) (* (+ (Variables|Default|GetRank1Rate) (Variables|Default|GetRank2Rate) (Variables|Default|GetRank3Rate)) -1.0))))

(fn ConstructionScript)