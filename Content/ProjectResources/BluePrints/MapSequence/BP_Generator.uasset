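; Generator actor for the map sequence that has a cable and a switchable on/off state.
; On BeginPlay it attaches the cable's end to the CableAttatch socket on the StaticMesh component of the ActorForCable actor.
; TogglePower flips IsOn and shows or hides four cylinder components to match, with no other effect in this graph.
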(event EventBeginPlay
  (Class|CableComponent|SetAttachEndto (Variables|Default|GetCable) (Variables|Default|GetActorForCable) "StaticMesh" "CableAttatch"))

(event Collision|EventActorBeginOverlap
  (params (OtherActor :type Actor%20Object%20Reference)))

(event EventTick
  (params (DeltaSeconds :type Float%20%28single-precision%29)))

(event EventTogglePower
  (bind _cylinder (Variables|Default|GetCylinder))
  (if (Variables|Default|GetbIsOn?)
    (Rendering|SetVisibility _cylinder false false)
    (Variables|Default|SetbIsOn? false)
    (else
      (Rendering|SetVisibility _cylinder true false)
      (Variables|Default|SetbIsOn? true))))

(fn ConstructionScript)