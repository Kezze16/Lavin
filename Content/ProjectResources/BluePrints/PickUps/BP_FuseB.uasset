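; BP_FuseB is a fuse pickup that, on Interact, adds itself as an item to the player's BPC_Inventory and triggers power-off effects.
; It plays the PowerOff sound at its location and pushes a sound mix override that silences the PowerOffSoundsB class.
; It then hides each actor in ActorsToHide, destroying ActorsToDestroy and itself inside that loop, so destruction depends on ActorsToHide being non-empty.
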(event EventInteract
  (Default|AddInventoryItem (Actor|GetComponentbyClass (Game|GetPlayerCharacter 0) "/Game/ProjectResources/BluePrints/Inventory/BPC_Inventory.BPC_Inventory_C") "NewEnumerator8")
  (Audio|PlaySoundatLocation "/Game/ProjectResources/Sound/SFX/PowerOff.PowerOff" (Transformation|GetActorLocation) "0, 0, 0" 1.0 1.0 0.0 0 0 0 0)
  (Audio|SetSoundMixClassOverride "/Game/ProjectResources/Sound/SoundClass/MasterSoundMix.MasterSoundMix" "/Game/ProjectResources/Sound/SoundClass/PowerOffSoundsB.PowerOffSoundsB" 0.0 1.0 1.0 true)
  (Audio|PushSoundMixModifier "/Game/ProjectResources/Sound/SoundClass/MasterSoundMix.MasterSoundMix")
  (for _array_element (Variables|Default|GetActors%20to%20Hide)
    (Rendering|SetActorHiddenInGame _array_element true)
    (Actor|DestroyActor (Variables|Default|GetActors%20to%20Destroy))))

(fn ConstructionScript)