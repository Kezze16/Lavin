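; BP_KnifeHandle is a pickup actor that puts an item, presumably the knife handle, into the player's inventory.
; Its Interact event finds the BPC_Inventory component on player character 0, adds a fixed enum-identified item and then destroys the actor.
; BeginPlay, overlap and Tick are disabled, so Interact is the only active logic.
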(event EventBeginPlay
  (|CallParentFunction) ; This node is disabled and will not be called.\nDrag off pins to build functionality.
)

(event Collision|EventActorBeginOverlap
  (params (OtherActor :type Actor%20Object%20Reference))
  (|CallParentFunction OtherActor) ; This node is disabled and will not be called.\nDrag off pins to build functionality.
)

(event EventTick
  (params (DeltaSeconds :type Float%20%28single-precision%29))
  (|CallParentFunction DeltaSeconds) ; This node is disabled and will not be called.\nDrag off pins to build functionality.
)

(event EventInteract
  (Default|AddInventoryItem (Actor|GetComponentbyClass (Game|GetPlayerCharacter 0) "/Game/ProjectResources/BluePrints/Inventory/BPC_Inventory.BPC_Inventory_C") "NewEnumerator4")
  (Actor|DestroyActor))

(fn ConstructionScript
  (|CallParentFunction))